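; Fire projectile actor that damages third-person characters it hits and bursts into an Explosion actor.
; A timer calls Explode after a fixed lifetime, spawning the explosion at the projectile's transform and destroying the projectile.
; Hit reacts only to ThirdPersonCharacter actors whose Name is not "Char01", calling Explode and then applying damage; other hits are ignored.
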(event EventBeginPlay
  (Utilities|Time|SetTimerbyFunctionName 0 "Explode" 5.0))

(event EventActorBeginOverlap
  (params (OtherActor :type Actor%20Object%20Reference)))

(event EventTick
  (params (DeltaSeconds :type Float%20%28single-precision%29)))

(event Collision|EventHit
  (params (MyComp :type Primitive%20Component%20Object%20Reference) (Other :type Actor%20Object%20Reference) (OtherComp :type Primitive%20Component%20Object%20Reference) (bSelfMoved :type Boolean) (HitLocation :type Vector :default "0, 0, 0") (HitNormal :type Vector :default "0, 0, 0") (NormalImpulse :type Vector :default "0, 0, 0") (Hit :type Hit%20Result%20Structure%20%28by%20ref%29))
  (bind _asthird_person_character (Utilities|Casting|CastToThirdPersonCharacter Other))
  (if (not (Utilities|Enum|Equal(Enum) (Variables|/Game/Blueprints/Chars/ThirdPersonCharacter.ThirdPersonCharacter_C|Getname _asthird_person_character) "Char01"))
    (CallFunction|Explode)
    (Game|Damage|ApplyDamage _asthird_person_character 2e+01 0 0)))

(fn ConstructionScript)

(fn Explode
  (Game|SpawnActorfromClass "/Game/Blueprints/Explosion.Explosion_C" (Transformation|GetActorTransform) "Undefined" 0 self)
  (Actor|DestroyActor))